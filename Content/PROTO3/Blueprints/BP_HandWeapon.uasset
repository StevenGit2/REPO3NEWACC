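; Hand-held weapon Blueprint that fires FirstPersonProjectile from a transform passed to its Attack event.
; Tick runs a cooldown timer that restores CanAttack, but Attack itself neither checks that flag nor calls UseAmmo, which decrements ammo down to zero.
; The construction script tints the skeletal mesh from Color.
; AddToHUD creates the BP_GameHUD widget, while RemoveFromHUD does nothing because its removal node is disconnected.
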(event `self.ReceiveTick`
  (params (DeltaSeconds :type "Float (single-precision)"))
  (if (`self.CanAttack`)
    _
    (elif (>= (`self.AttackTimer`) (`self.AttackCooldown`))
      (set `self.CanAttack` true)
      (set `self.AttackTimer` 0.0)
      (else
        (set `self.AttackTimer` (+ (`self.AttackTimer`) DeltaSeconds))))))

(event `Attack`
  (params (SpawnTransform :type "Transform Structure"))
  (`|SpawnActorFromClass` "/Game/FirstPersonBP/Blueprints/FirstPersonProjectile.FirstPersonProjectile_C" SpawnTransform "AdjustIfPossibleButDontSpawnIfColliding" "OverrideRootScale" null null) ; Spawn projectile
)

(event `AddToHUD`
  (bind _returnvalue (`|CreateWidget` "/Game/PROTO3/UI/BP_GameHUD.BP_GameHUD_C" (`GameplayStatics.GetPlayerController` 0)))
  (set `self.BaseWidget` _returnvalue)
  (`UserWidget.AddToViewport` _returnvalue 0))

(event `self.ReceiveEndPlay`
  (params (EndPlayReason :type "EEndPlayReason Enum" :default "Destroyed")))

(fn `RemoveFromHUD`)

(fn `UseAmmo`
  (if (> (`self.CurrentAmmo`) 0)
    (set `self.CurrentAmmo` (- (`self.CurrentAmmo`) 1))
    (else
      (set `self.CurrentAmmo` 0))))

(fn `UserConstructionScript`
  (`MeshComponent.SetVectorParameterValueOnMaterials` (`self.SkeletalMesh`) "BodyColor" (`KismetMathLibrary.Conv_LinearColorToVector` (`self.Color`))))