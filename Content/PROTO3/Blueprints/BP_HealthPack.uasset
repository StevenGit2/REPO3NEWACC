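; Health pack item that occupies a slot in the player's weapon array and heals on attack, using the parent class's ammo as charges.
; HealPlayer spends a charge only below max HP, clamps the result, plays a sound and clears CanAttack.
; When charges run out, RemoveFromPlayer drops it from the array, equips from index 1, removes its HUD widget and destroys the parent actor.
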(event `self.ReceiveBeginPlay`
  (`parent.ReceiveBeginPlay`)
  (set `self.CurrentAmmo` 2)
  (set `self.MaxAmmo` 10)
  (set `self.AttackCooldown` 1.0))

(event `self.Attack`
  (params (SpawnTransform :type "Transform Structure"))
  (if (`self.CanAttack`)
    (`self.HealPlayer`)
    (if (<= (`self.CurrentAmmo`) 0)
      (`self.RemoveFromPlayer`))))

(event `self.AddToHUD`
  (`parent.AddToHUD`)
  (bind _returnvalue (`|CreateWidget` "/Game/PROTO3/UI/BP_HealPackUI.BP_HealPackUI_C" (`GameplayStatics.GetPlayerController` 0)))
  (`UserWidget.AddToViewport` _returnvalue 0)
  (set `self.SecondaryWidget` _returnvalue))

(fn `HealPlayer`
  (bind _asbp_player (cast `/Game/PROTO3/Blueprints/BP_Player` (`GameplayStatics.GetPlayerCharacter` 0)))
  (if (< (`/Game/PROTO3/Blueprints/BP_Player.CurrentHP` _asbp_player) (`/Game/PROTO3/Blueprints/BP_Player.MaxHP` _asbp_player))
    (`self.UseAmmo`)
    (bind _output_get (set `/Game/PROTO3/Blueprints/BP_Player.CurrentHP` (+ (`/Game/PROTO3/Blueprints/BP_Player.CurrentHP` _asbp_player) (`self.HealthPerUse`)) _asbp_player))
    (`GameplayStatics.PlaySound2D` "/Game/PROTO3/Audio/heal.heal" 1.0 1.0 0.0 null null)
    (set `self.CanAttack` false)
    (bind _maxhp (`/Game/PROTO3/Blueprints/BP_Player.MaxHP` _asbp_player))
    (if (not (< _output_get _maxhp))
      (set `/Game/PROTO3/Blueprints/BP_Player.CurrentHP` _maxhp _asbp_player))))

(fn `RemoveFromPlayer`
  (bind _asbp_player (cast `/Game/PROTO3/Blueprints/BP_Player` (`GameplayStatics.GetPlayerCharacter` 0)))
  (bind _weaponarray (`/Game/PROTO3/Blueprints/BP_Player.WeaponArray` _asbp_player))
  (bind _returnvalue (`KismetArrayLibrary.Array_RemoveItem` _weaponarray (`|GetArrayItem` _weaponarray (`/Game/PROTO3/Blueprints/BP_Player.CurrentWeaponIndex` _asbp_player))))
  (`KismetSystemLibrary.PrintString` "removed" _returnvalue)
  (set `/Game/PROTO3/Blueprints/BP_Player.CurrentWeaponIndex` 1 _asbp_player)
  (`/Game/PROTO3/Blueprints/BP_Player.EquipWeapon` _asbp_player _weaponarray)
  (`Widget.RemoveFromParent` (`self.SecondaryWidget`))
  (`self.K2_DestroyActor` (`self.GetParentActor`)))

(fn `UserConstructionScript`
  (`parent.UserConstructionScript`))