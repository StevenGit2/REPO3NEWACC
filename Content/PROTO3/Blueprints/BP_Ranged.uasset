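; Ranged weapon Blueprint that fires BP_Projectile actors, building on a parent class with a short attack cooldown set at BeginPlay.
; Attack checks CanAttack and remaining ammo, spawns the projectile at the supplied transform, calls UseAmmo, then clears CanAttack; nothing here re-enables it.
; AddtoHUD extends the parent's HUD setup by adding a BP_RangedWeaponUI widget to the viewport and storing it as SecondaryWidget.
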(event `self.Attack`
  (params (SpawnTransform :type "Transform Structure"))
  (if (`self.CanAttack`)
    (if (> (`self.CurrentAmmo`) 0)
      (`|SpawnActorFromClass` "/Game/PROTO3/Blueprints/BP_Projectile.BP_Projectile_C" SpawnTransform "AdjustIfPossibleButDontSpawnIfColliding" "OverrideRootScale" null null) ; Spawn projectile
      (`self.UseAmmo`)
      (set `self.CanAttack` false))))

(event `self.ReceiveBeginPlay`
  (`parent.ReceiveBeginPlay`)
  (set `self.AttackCooldown` 0.1))

(event `self.AddToHUD`
  (`parent.AddToHUD`)
  (bind _returnvalue (`|CreateWidget` "/Game/PROTO3/UI/BP_RangedWeaponUI.BP_RangedWeaponUI_C" (`GameplayStatics.GetPlayerController` 0)))
  (`UserWidget.AddToViewport` _returnvalue 0)
  (set `self.SecondaryWidget` _returnvalue))

(fn `UserConstructionScript`
  (`parent.UserConstructionScript`))