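; BP_EndTrigger is an overlap trigger that ends the game once the player has completed the journal.
; On actor overlap it casts to BP_Player and checks HasCompletedJournal, doing nothing otherwise.
; When the check passes, it clears sound mix modifiers, plays the end boss sound, shows a fade-to-black widget, then after a short delay opens the end menu level.
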(event `self.ReceiveActorBeginOverlap`
  (params (OtherActor :type "Actor Object Reference"))
  (bind _asbp_player (cast `/Game/PROTO3/Blueprints/BP_Player` OtherActor))
  (bind _hascompleted (`/Game/PROTO3/Blueprints/BP_Player.HasCompletedJournal` _asbp_player))
  (if _hascompleted
    (`GameplayStatics.ClearSoundMixModifiers`)
    (`GameplayStatics.PlaySound2D` "/Game/PROTO3/Audio/endBossSFX.endBossSFX" 1.0 1.0 0.0 null null)
    (bind _returnvalue (`|CreateWidget` "/Game/PROTO3/UI/BP_FadeToBlack.BP_FadeToBlack_C" (`GameplayStatics.GetPlayerController` 0)))
    (`UserWidget.AddToViewport` _returnvalue 0)
    (`/Game/PROTO3/UI/BP_FadeToBlack.Fade To Black` _returnvalue)
    (`KismetSystemLibrary.Delay` 4.0)
    (`GameplayStatics.OpenLevelBySoftObjectPtr` "/Game/PROTO3/Maps/EndMenu.EndMenu")))

(fn `UserConstructionScript`)