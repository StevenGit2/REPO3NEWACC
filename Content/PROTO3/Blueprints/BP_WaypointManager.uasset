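; Waypoint manager Blueprint that steps through an ordered WaypointList, keeping the first unreached waypoint active.
; BeginPlay deactivates every waypoint, including the first despite its "true" debug print.
; Each Tick scans the list in order, deactivating reached waypoints and activating the first unreached one before stopping, so progression relies on polling each waypoint's Reached flag.
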(event `self.ReceiveBeginPlay`
  (for (_array_element _array_index) (`self.WaypointList`)
    (if (== _array_index 0)
      (set `/Game/PROTO3/Blueprints/BP_Waypoint.IsActive` false _array_element)
      (`KismetSystemLibrary.PrintString` "true")
      (else
        (set `/Game/PROTO3/Blueprints/BP_Waypoint.IsActive` false _array_element)
        (`KismetSystemLibrary.PrintString` "set false")))))

(event `self.ReceiveActorBeginOverlap`
  (params (OtherActor :type "Actor Object Reference")))

(event `self.ReceiveTick`
  (params (DeltaSeconds :type "Float (single-precision)"))
  (for _array_element (`self.WaypointList`)
    (if (`/Game/PROTO3/Blueprints/BP_Waypoint.Reached` _array_element)
      (set `/Game/PROTO3/Blueprints/BP_Waypoint.IsActive` false _array_element)
      (else
        (set `/Game/PROTO3/Blueprints/BP_Waypoint.IsActive` true _array_element)
        (break)))))

(fn `UserConstructionScript`)