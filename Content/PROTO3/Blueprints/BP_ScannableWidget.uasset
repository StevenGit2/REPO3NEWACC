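; BP_ScannableWidget is an actor that bobs and spins in place; despite its name, it holds no scanning logic.
; Each Tick adds a small sine-of-lifetime offset to the root's current world Z, written back as relative location, and applies a fixed rotation step.
; Because the offsets accumulate and neither step uses DeltaSeconds, bob height and spin speed depend on frame rate.
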(event `self.ReceiveTick`
  (params (DeltaSeconds :type "Float (single-precision)"))
  (bind (_returnvalue_x _returnvalue_y _returnvalue_z) (`KismetMathLibrary.BreakVector` (`SceneComponent.K2_GetComponentLocation` (`self.DefaultSceneRoot`))))
  (`parent.ReceiveTick` DeltaSeconds)
  (`self.K2_SetActorRelativeLocation` (`KismetMathLibrary.MakeVector` _returnvalue_x _returnvalue_y (+ (* (`KismetMathLibrary.DegSin` (* (`self.GetGameTimeSinceCreation`) 100.0)) 0.2) _returnvalue_z)))
  (`SceneComponent.K2_AddRelativeRotation` (`self.DefaultSceneRoot`) (struct :`Yaw` 0.2) false false))

(fn `UserConstructionScript`
  (`parent.UserConstructionScript`))