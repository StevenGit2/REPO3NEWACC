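; BP_Melee is a child weapon Blueprint whose Attack damages flying AI enemies.
; When CanAttack is set, a debug-drawn line trace runs forward from FirePoint and applies Damage to FlyingAI Ver1 or Ver2 hits.
; Attack then clears CanAttack, except on a Ver3 hit, which does nothing.
; BeginPlay sets AttackCooldown, with no reset here, and an unused sphere-overlap branch remains disconnected.
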(event `self.Attack`
  (params (SpawnTransform :type "Transform Structure"))
  (bind _damage (`self.Damage`))
  (bind _firepoint (`self.FirePoint`))
  (bind _returnvalue (`SceneComponent.K2_GetComponentLocation` _firepoint))
  (if (`self.CanAttack`)
    (bind _outhit (`KismetSystemLibrary.LineTraceSingle` :`Start` _returnvalue :`End` (+ _returnvalue (* (`KismetMathLibrary.GetForwardVector` (`SceneComponent.K2_GetComponentRotation` _firepoint)) 1000.0)) :`TraceChannel` "TraceTypeQuery1" :`bTraceComplex` true :`DrawDebugType` "ForDuration"))
    (bind (_bblockinghit _binitialoverlap _time _distance _location _impactpoint _normal _impactnormal _physmat _hitactor) (`GameplayStatics.BreakHitResult` _outhit))
    (bind _asflying_ai_ver_1 (cast `/Game/PROTO3/AI/FlyingAI_Ver1` _hitactor)
      (:`then`
        (`/Game/PROTO3/AI/FlyingAI_Ver1.TakeDamage` _asflying_ai_ver_1 _damage))
      (:`CastFailed`
        (bind _asflying_ai_ver_2 (cast `/Game/PROTO3/AI/FlyingAi_Ver2` _hitactor)
          (:`then`
            (`/Game/PROTO3/AI/FlyingAi_Ver2.TakeDamage` _asflying_ai_ver_2 _damage))
          (:`CastFailed`
            (cast `/Game/PROTO3/AI/FlyingAI_Ver3` _hitactor
              (:`CastFailed`
                _))))))
    (set `self.CanAttack` false)))

(event `self.ReceiveBeginPlay`
  (`parent.ReceiveBeginPlay`)
  (set `self.AttackCooldown` 0.5))

(event `self.AddToHUD`
  ;[1 1 1] Override
  (`parent.AddToHUD`))

(fn `UserConstructionScript`
  (`parent.UserConstructionScript`))