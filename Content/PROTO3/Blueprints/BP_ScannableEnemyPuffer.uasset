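; Scannable pufferfish enemy that supplies its own scan data and removes itself after a fixed lifetime.
; On BeginPlay, if the scan name is still "???", it loads the Puffer row from DT_Scannable into ScanData and sets the fish spike material as OGMaterial, without calling parent BeginPlay.
; Tick runs the parent logic, then a 15-second Delay leads to DestroyActor.
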(event `self.ReceiveBeginPlay`
  (bind _scandata_name (break `/Game/PROTO3/Blueprints/BP_ScanStruct` (`self.ScanData`)))
  (if (`KismetStringLibrary.EqualEqual_StrStr` _scandata_name "???")
    (bind _returnvalue (`|GetDataTableRow` "/Game/PROTO3/Blueprints/DT_Scannable.DT_Scannable" "Puffer")
      (:`then`
        (set `self.ScanData` _returnvalue)
        (set `self.OGMaterial` "/Game/PROTO3/Material/Fish/M_FishSpike.M_FishSpike")))))

(event `self.ReceiveTick`
  (params (DeltaSeconds :type "Float (single-precision)"))
  (`parent.ReceiveTick` DeltaSeconds)
  (`KismetSystemLibrary.Delay` 15.0)
  (`self.K2_DestroyActor`))

(fn `UserConstructionScript`
  (`parent.UserConstructionScript`))