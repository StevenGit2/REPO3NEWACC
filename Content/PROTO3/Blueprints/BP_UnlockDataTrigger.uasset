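; BP_UnlockDataTrigger is a trigger that unlocks a named entry in the player's scanned data when the player overlaps it.
; On actor overlap it casts to BP_Player, loops through the ScannedData array and compares each entry's Name to its DataName variable.
; Each match is set to unlocked in place through a by-ref write, and DataName is printed as debug output.
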(event `self.ReceiveActorBeginOverlap`
  (params (OtherActor :type "Actor Object Reference"))
  (bind _asbp_player (cast `/Game/PROTO3/Blueprints/BP_Player` OtherActor))
  (bind _scanneddata (`/Game/PROTO3/Blueprints/BP_Player.ScannedData` _asbp_player))
  (for (_array_element _array_index) _scanneddata
    (if (== (break `/Game/PROTO3/Blueprints/BP_ScannedDataStruct` _array_element) (`self.DataName`))
      (bind _output_name (break `/Game/PROTO3/Blueprints/BP_ScannedDataStruct` (`|GetArrayItem` _scanneddata _array_index)))
      (`|VariableSetRef` (`|GetArrayItem` _scanneddata _array_index) (make `/Game/PROTO3/Blueprints/BP_ScannedDataStruct` _output_name true))
      (`KismetSystemLibrary.PrintString` (`self.DataName`)))))

(fn `UserConstructionScript`)