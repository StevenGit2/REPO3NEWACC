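; BP_CausticSwitch is a volume actor that switches the player between dry walking and underwater swimming, along with the matching lighting.
; Play start and player entry hide the fog, clear the directional light's function material, dim it and, after a short delay, start walk controls.
; Player exit shows the fog, applies a caustics light function at high intensity and, after a shorter delay, starts swim controls.
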(event `self.ReceiveBeginPlay`
  (bind _lightcomponent (`Light.LightComponent` (`self.DirLight`)))
  (`SceneComponent.SetVisibility` (`ExponentialHeightFog.Component` (`self.Fog`)) false false :!label _label)
  (`LightComponent.SetLightFunctionMaterial` _lightcomponent null)
  (`LightComponent.SetIntensity` _lightcomponent 1.0)
  (`KismetSystemLibrary.Delay` 0.3)
  (bind _asbp_player (cast `/Game/PROTO3/Blueprints/BP_Player` (`GameplayStatics.GetPlayerCharacter` 0)))
  (`/Game/PROTO3/Blueprints/BP_Player.StartWalkControls` _asbp_player))

(event `self.ReceiveActorEndOverlap`
  (params (OtherActor :type "Actor Object Reference"))
  (bind _lightcomponent (`Light.LightComponent` (`self.DirLight`)))
  (cast `/Game/PROTO3/Blueprints/BP_Player` OtherActor)
  (`SceneComponent.SetVisibility` (`ExponentialHeightFog.Component` (`self.Fog`)) true false)
  (`LightComponent.SetLightFunctionMaterial` _lightcomponent "/Game/PROTO3/Material/M_Caustics_Inst.M_Caustics_Inst")
  (`LightComponent.SetIntensity` _lightcomponent 150.0)
  (`KismetSystemLibrary.Delay` 0.05)
  (bind _asbp_player (cast `/Game/PROTO3/Blueprints/BP_Player` (`GameplayStatics.GetPlayerCharacter` 0)))
  (`/Game/PROTO3/Blueprints/BP_Player.StartSwimControls` _asbp_player))

(event `self.ReceiveActorBeginOverlap`
  (params (OtherActor :type "Actor Object Reference"))
  (cast `/Game/PROTO3/Blueprints/BP_Player` OtherActor)
  (goto _label))

(fn `UserConstructionScript`)