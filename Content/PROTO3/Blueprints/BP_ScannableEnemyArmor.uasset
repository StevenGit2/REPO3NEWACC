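; BP_ScannableEnemyArmor is a scannable enemy armor actor that removes itself about ten seconds after it starts ticking.
; On BeginPlay, it fills ScanData from the Enemy2 row of DT_Scannable if the name is still the "???" placeholder, without calling parent BeginPlay.
; Tick calls the parent, then uses a Delay before DestroyActor as a simple lifespan timer.
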(event `self.ReceiveBeginPlay`
  (bind _scandata_name (break `/Game/PROTO3/Blueprints/BP_ScanStruct` (`self.ScanData`)))
  (if (`KismetStringLibrary.EqualEqual_StrStr` _scandata_name "???")
    (bind _returnvalue (`|GetDataTableRow` "/Game/PROTO3/Blueprints/DT_Scannable.DT_Scannable" "Enemy2")
      (:`then`
        (set `self.ScanData` _returnvalue)))))

(event `self.ReceiveTick`
  (params (DeltaSeconds :type "Float (single-precision)"))
  (`parent.ReceiveTick` DeltaSeconds)
  (`KismetSystemLibrary.Delay` 10.0)
  (`self.K2_DestroyActor`))

(fn `UserConstructionScript`
  (`parent.UserConstructionScript`))