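; BP_HealPackTrigger is a world pickup that gives the player a health pack weapon on overlap.
; It searches the player's WeaponArray for an existing BP_HealthPack; if found, it tops up that pack's ammo and destroys itself.
; Otherwise it adds its child actor component to the array, attaches it to the Mesh2P grip socket and equips it.
; It then hides its static mesh and sets Detached to block repeat pickups.
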(event `self.ReceiveActorBeginOverlap`
  (params (OtherActor :type "Actor Object Reference"))
  (bind _childactor (`self.ChildActor`))
  (bind _asbp_player (cast `/Game/PROTO3/Blueprints/BP_Player` OtherActor))
  (if (not (`self.Detached`))
    (for (_array_element _array_index) (`/Game/PROTO3/Blueprints/BP_Player.WeaponArray` _asbp_player)
      (bind _asbp_health_pack (cast `/Game/PROTO3/Blueprints/BP_HealthPack` (`ChildActorComponent.ChildActor` _array_element)))
      (set `self.HealthPackOwned` true)
      (set `self.HealthpackIndex` _array_index)
      (break))
    (if (`self.HealthPackOwned`)
      (set `/Game/PROTO3/Blueprints/BP_HandWeapon.CurrentAmmo` (+ (`/Game/PROTO3/Blueprints/BP_HandWeapon.CurrentAmmo` _asbp_health_pack) 2) _asbp_health_pack)
      (`self.K2_DestroyActor`)
      (else
        (bind _weaponarray (`/Game/PROTO3/Blueprints/BP_Player.WeaponArray` _asbp_player))
        (bind _returnvalue (`KismetArrayLibrary.Array_Add` _weaponarray _childactor))
        (`SceneComponent.K2_AttachToComponent` _childactor (`/Game/PROTO3/Blueprints/BP_Player.Mesh2P` _asbp_player) "GripPoint" "SnapToTarget" "SnapToTarget" "SnapToTarget" true)
        (set `/Game/PROTO3/Blueprints/BP_Player.CurrentWeaponIndex` _returnvalue _asbp_player)
        (`/Game/PROTO3/Blueprints/BP_Player.EquipWeapon` _asbp_player _weaponarray)
        (`SceneComponent.SetVisibility` (`self.ChildActor`) true false)
        (`KismetSystemLibrary.PrintString` "health pack picked up\\")
        (set `self.Detached` true)
        (`SceneComponent.SetVisibility` (`self.StaticMesh`) false false)))))

(fn `UserConstructionScript`)