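; BP_RangedAmmoTrigger is a spinning ammo pickup for the player's ranged weapons.
; On overlap with BP_Player, it loops over WeaponArray and adds AmmoToGive to CurrentAmmo on each BP_Ranged child actor.
; The pickup sound and DestroyActor sit inside the loop, so they fire per ranged weapon, and the pickup remains if none is found.
; Tick applies a fixed local rotation every frame, independent of delta time.
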(event `self.ReceiveActorBeginOverlap`
  (params (OtherActor :type "Actor Object Reference"))
  (bind _asbp_player (cast `/Game/PROTO3/Blueprints/BP_Player` OtherActor))
  (for _array_element (`/Game/PROTO3/Blueprints/BP_Player.WeaponArray` _asbp_player)
    (bind _asbp_ranged (cast `/Game/PROTO3/Blueprints/BP_Ranged` (`ChildActorComponent.ChildActor` _array_element)))
    (set `/Game/PROTO3/Blueprints/BP_HandWeapon.CurrentAmmo` (+ (`/Game/PROTO3/Blueprints/BP_HandWeapon.CurrentAmmo` _asbp_ranged) (`self.AmmoToGive`)) _asbp_ranged)
    (`GameplayStatics.PlaySound2D` "/Game/PROTO3/Audio/itempick.itempick" 1.0 1.0 0.0 null null)
    (`self.K2_DestroyActor`)))

(event `self.ReceiveTick`
  (params (DeltaSeconds :type "Float (single-precision)"))
  (`self.K2_AddActorLocalRotation` (struct :`Yaw` 1.0)))

(fn `UserConstructionScript`)