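; Bullet_BP is a projectile actor in the PROTO3 AI folder that damages the player on impact.
; Its Hit event casts the hit actor to BP_Player and calls TakeDamage with its Damage value.
; It then destroys itself unless the other actor matches FlyingAI_Ver1, likely the shooter.
; Tick accumulates SurviveTime and destroys the bullet after a five-second lifetime.
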(event `self.ReceiveHit`
  (params (MyComp :type "PrimitiveComponent Object Reference") (Other :type "Actor Object Reference") (OtherComp :type "PrimitiveComponent Object Reference") (bSelfMoved :type Boolean) (HitLocation :type "Vector Structure") (HitNormal :type "Vector Structure") (NormalImpulse :type "Vector Structure") (Hit :type "HitResult Structure (by ref)"))
  (`|ExecutionSequence`
    (:`then_0`
      (bind _asbp_player (cast `/Game/PROTO3/Blueprints/BP_Player` (`.HitActor` (`GameplayStatics.BreakHitResult` Hit))))
      (`/Game/PROTO3/Blueprints/BP_Player.TakeDamage` _asbp_player (`self.Damage`)))
    (:`then_1`
      (if (not (== Other "/Game/PROTO3/AI/FlyingAI_Ver1.FlyingAI_Ver1"))
        (`self.K2_DestroyActor`)))))

(event `self.ReceiveActorBeginOverlap`
  (params (OtherActor :type "Actor Object Reference")))

(event `self.ReceiveTick`
  (params (DeltaSeconds :type "Float (single-precision)"))
  (set `self.SurviveTime` (+ (`self.SurviveTime`) DeltaSeconds))
  (if (>= (`self.SurviveTime`) 5.0)
    (`self.K2_DestroyActor`)))

(fn `UserConstructionScript`)